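; BP_SplinePathForSnake is a spline path actor, named for a snake, that visualizes its route at runtime.
; On BeginPlay, DrawSnakeDebugLine samples the spline in world space at StepCount evenly spaced distances along its length.
; Consecutive samples are joined with thick, long-lasting colored debug lines, approximating the curve as straight segments.
; The file contains no movement logic; its overlap, tick and construction script graphs are empty.
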(event EventBeginPlay
  (CallFunction|DrawSnakeDebugLine))

(event Collision|EventActorBeginOverlap
  (params (OtherActor :type Actor%20Object%20Reference)))

(event EventTick
  (params (DeltaSeconds :type Float%20%28single-precision%29)))

(fn ConstructionScript)

(fn DrawSnakeDebugLine
  (bind _spline (Variables|Default|GetSpline))
  (bind _stepcount (LocalVariables|GetStepCount))
  (LocalVariables|SetTmpVec (Spline|GetLocationatDistanceAlongSpline _spline 0.0 "World"))
  (for _index (range 1 _stepcount)
    (Rendering|Debug|DrawDebugLine (LocalVariables|GetTmpVec) (Spline|GetLocationatDistanceAlongSpline (Variables|Default|GetSpline) (* (Spline|GetSplineLength _spline) (/ (Math|Conversions|ToFloat(Integer) _index) (Math|Conversions|ToFloat(Integer) _stepcount))) "World") "(R=1.000000,G=0.000000,B=0.808993,A=1.000000)" 6e+02 16.0)
    (LocalVariables|SetTmpVec (Spline|GetLocationatDistanceAlongSpline (Variables|Default|GetSpline) (* (Spline|GetSplineLength _spline) (/ (Math|Conversions|ToFloat(Integer) _index) (Math|Conversions|ToFloat(Integer) _stepcount))) "World"))))