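; BP_FlyPawn is a pawn with rough debug-key tests for vertical flight through FloatingPawnMovement.
; Pressing W, or calling the AAA event, adds one large input vector along the actor's up vector; releasing W adds a smaller downward one.
; Debug prints report the up vector, acceleration and key states, while S only prints.
; Tick is empty and the forward-movement, offset and acceleration experiments are left disconnected.
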(event Custom|AAA
  (bind _returnvalue (Transformation|GetActorUpVector))
  (Class|PawnMovementComponent|AddInputVector (Variables|Default|GetFloatingPawnMovement) (* _returnvalue 4e+03) false)
  (Development|PrintString (Utilities|String|ToString(Vector) _returnvalue)))

(event EventBeginPlay)

(event Collision|EventActorBeginOverlap
  (params (OtherActor :type Actor%20Object%20Reference)))

(event EventTick
  (params (DeltaSeconds :type Float%20%28single-precision%29)))

(event Input|KeyboardEvents|DebugKeyComboKey
  (params (Key :type Key%20Structure :default "None") (ActionValue :type Input%20Action%20Value%20Structure)))

(event Input|KeyboardEvents|DebugKeyW
  (params (Key :type Key%20Structure :default "None") (ActionValue :type Input%20Action%20Value%20Structure))
  (bind _returnvalue (Transformation|GetActorUpVector))
  (:Pressed
    (Class|PawnMovementComponent|AddInputVector (Variables|Default|GetFloatingPawnMovement) (* _returnvalue 4e+03) false)
    (Development|PrintString (Utilities|String|ToString(Vector) _returnvalue)))
  (:Released
    (Development|PrintString "w r")
    (Development|PrintString (Utilities|String|ToString(Float) (Variables|/Script/Engine.FloatingPawnMovement|GetAcceleration (Variables|Default|GetFloatingPawnMovement))))
    (Class|PawnMovementComponent|AddInputVector (Variables|Default|GetFloatingPawnMovement) (* (Transformation|GetActorUpVector) -9.8e+02) false)))

(event Input|KeyboardEvents|DebugKeyS
  (params (Key :type Key%20Structure :default "None") (ActionValue :type Input%20Action%20Value%20Structure))
  (:Pressed
    (Development|PrintString "s d"))
  (:Released
    (Development|PrintString "s r")))

(fn ConstructionScript)