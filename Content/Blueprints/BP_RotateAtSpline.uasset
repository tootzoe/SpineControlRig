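; Spline actor that can snap its points to the ground and holds unfinished experiments for driving a BP_RotatorActor along the path.
; BeginPlay caches the first rotator actor found.
; SnapSplineToGround line-traces down from each spline point on the Visibility channel and moves hit points just above the surface.
; Logic for moving and rotating the cached actor along the spline is disconnected, so it never runs.
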(event Custom|SnapSplineToGround
  (bind _spline (Variables|Default|GetSpline))
  (for _index (range 0 (Spline|GetNumberOfSplinePoints _spline))
    (bind (_outhit _returnvalue) (Collision|LineTraceByChannel (Spline|GetLocationatSplinePoint _spline _index "World") (+ (Spline|GetLocationatSplinePoint _spline _index "World") (Math|Vector|MakeVector 0.0 0.0 (* (Variables|Default|GetTraceDistacne) -1.0))) "TraceTypeQuery1" false 0 "ForDuration"))
    (if _returnvalue
      (Spline|SetLocationatSplinePoint _spline _index (+ (.Location (Collision|BreakHitResult _outhit)) (Math|Vector|MakeVector 0.0 0.0 2e+01)) "World" true))))

(event EventBeginPlay
  (bind _returnvalue (Actor|GetActorOfClass "/Game/Blueprints/BP_RotatorActor.BP_RotatorActor_C"))
  (Variables|Default|SetTootRot _returnvalue))

(event Collision|EventActorBeginOverlap
  (params (OtherActor :type Actor%20Object%20Reference)))

(event EventTick
  (params (DeltaSeconds :type Float%20%28single-precision%29)))

(fn ConstructionScript)