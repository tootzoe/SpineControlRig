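; BP_DynSpline is a test actor for editing and visualizing a spline component at runtime.
; Each Tick loops over all points, drawing debug axes at half-tangent offsets on either side.
; The same loop spins point 1's up vector via an accumulating roll, so speed scales with point count, and draws and prints the result.
; Custom events add hard-coded points, remove the first point or print the point count.
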(event Custom|SEvt
  (Development|PrintString (Utilities|String|ToString(Integer) (Spline|GetNumberOfSplinePoints (Variables|Default|GetSpline)))))

(event Custom|AEvt
  (Spline|AddSplinePoint (Variables|Default|GetSpline) (Math|Vector|MakeVector 3e+02 6e+02 2e+02) "World" true))

(event Custom|AEvt2
  (Spline|AddSplinePoint (Variables|Default|GetSpline) (Math|Vector|MakeVector 2e+02 1e+03 2e+02) "World" true))

(event Custom|csp
  (Spline|RemoveSplinePoint (Variables|Default|GetSpline) 0 true))

(event EventBeginPlay)

(event Collision|EventActorBeginOverlap
  (params (OtherActor :type Actor%20Object%20Reference)))

(event EventTick
  (params (DeltaSeconds :type Float%20%28single-precision%29))
  (bind _spline (Variables|Default|GetSpline))
  (bind _spline_2 (Variables|Default|GetSpline))
  (bind _returnvalue (Spline|GetTransformatSplinePoint _spline_2 1 "World" false))
  (for _index (range 0 (- (Spline|GetNumberOfSplinePoints _spline) 1))
    (Class|KismetSystemLibrary|DrawDebugCoordinateSystem (+ (.Location (Spline|GetLocationandTangentatSplinePoint _spline _index "World")) (* (.Tangent (Spline|GetLocationandTangentatSplinePoint _spline _index "World")) 0.5)) "0, 0, 0" 1.0 2.0 1.0)
    (Class|KismetSystemLibrary|DrawDebugCoordinateSystem (- (.Location (Spline|GetLocationandTangentatSplinePoint _spline _index "World")) (* (.Tangent (Spline|GetLocationandTangentatSplinePoint _spline _index "World")) 0.5)) "0, 0, 0" 1.0 2.0 1.0)
    (Class|SplineComponent|SetUpVectoratSplinePoint _spline_2 1 (Math|Vector|RotateVector "0.000000,0.000000,90.000000" (Math|Rotator|MakeRotator (Variables|Default|GetMyRoll) 0.0 0.0)) "World" true)
    (Variables|Default|SetMyRoll (+ (Variables|Default|GetMyRoll) 2.0))
    (Class|KismetSystemLibrary|DrawDebugCoordinateSystem (.location _returnvalue) (.rotation _returnvalue) 33.0 2.0 1.0)
    (Development|PrintString (Utilities|String|ToString(Vector) (Class|SplineComponent|GetUpVectoratSplinePoint (Variables|Default|GetSpline) 1 "World")))))

(fn ConstructionScript)