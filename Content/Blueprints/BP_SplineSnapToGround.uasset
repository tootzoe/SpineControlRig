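; BP_SplineSnapToGround is a Blueprint utility that drops the points of its Spline1 component onto the surface below.
; The SnapSplineToGround event loops over the spline points in world space and line-traces straight down on the Visibility channel over a configurable distance, with timed debug drawing.
; On a hit, it moves the point to slightly above the impact; BeginPlay, Tick and the construction script do nothing.
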(event Custom|SnapSplineToGround
  (bind _spline1 (Variables|Default|GetSpline1))
  (for _index (range 0 (Spline|GetNumberOfSplinePoints _spline1))
    (bind (_outhit _returnvalue) (Collision|LineTraceByChannel (Spline|GetLocationatSplinePoint _spline1 _index "World") (+ (Spline|GetLocationatSplinePoint _spline1 _index "World") (Math|Vector|MakeVector 0.0 0.0 (* (Variables|Default|GetTraceDistacne) -1.0))) "TraceTypeQuery1" false 0 "ForDuration"))
    (if _returnvalue
      (Spline|SetLocationatSplinePoint _spline1 _index (+ (.Location (Collision|BreakHitResult _outhit)) (Math|Vector|MakeVector 0.0 0.0 3e+01)) "World" true))))

(event EventBeginPlay)

(event Collision|EventActorBeginOverlap
  (params (OtherActor :type Actor%20Object%20Reference)))

(event EventTick
  (params (DeltaSeconds :type Float%20%28single-precision%29)))

(fn ConstructionScript)