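; BP_3CrAxes is an actor that continuously orients itself toward the scene's BP_RotatorActor.
; BeginPlay finds and caches that actor, and Tick passes its location to LookAt, applying the resulting transform without sweep.
; The LookAt aims along the Z axis, which also serves as the up vector.
; An alternative Euler-to-quaternion rotation path and a debug print are left unconnected.
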(event EventBeginPlay
  (bind _returnvalue (Actor|GetActorOfClass "/Game/Blueprints/BP_RotatorActor.BP_RotatorActor_C"))
  (Variables|Default|SetRotActor _returnvalue))

(event Collision|EventActorBeginOverlap
  (params (OtherActor :type Actor%20Object%20Reference)))

(event EventTick
  (params (DeltaSeconds :type Float%20%28single-precision%29))
  (Transformation|SetActorTransform (Class|KismetAnimationLibrary|Lookat (Transformation|GetActorTransform) (Transformation|GetActorLocation (Variables|Default|GetRotActor)) "0.000000,0.000000,1.000000" false "0.000000,0.000000,1.000000" 0.0)))

(fn ConstructionScript)