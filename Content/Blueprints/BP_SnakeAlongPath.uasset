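; Snake actor Blueprint meant to drive a Control Rig snake skeletal mesh along a tagged spline path, though BeginPlay, Tick and MoveAlongPath are empty.
; Retrying finder events locate the spline and RIG_snakeAlongPath, but their calls are disconnected.
; Also disconnected: skeletal mesh mapping, plus a debug-drawn movement step that advances spline distance and inserts a tangent-derived transform at the front of the rig's spine-bone array.
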(event OnPreInitializeDelegate(ControlRig)
  (params (Component :type Control%20Rig%20Component%20Object%20Reference)))

(event Custom|FindSnakeRig
  (bind _returnvalue (Class|ControlRig|FindControlRigs (Variables|Default|GetControlRig) "/Game/Mesh/Snakes/SnakeAlongPath/RIG_snakeAlongPath.RIG_snakeAlongPath_C"))
  (if (Utilities|Array|IsNotEmpty _returnvalue)
    (bind _asrig_snake_along_path (Utilities|Casting|CastToRIG_snakeAlongPath (Utilities|Array|Get(acopy) _returnvalue)))
    (Variables|Default|SetSnakeRig _asrig_snake_along_path)
    (Development|PrintString "Found Snake Rig....")
    (else
      (Utilities|FlowControl|Delay 0.2)
      (CallFunction|FindSnakeRig))))

(event Custom|FindSnakePath
  (bind _outactors (Actor|GetAllActorsOfClasswithTag "/Game/Blueprints/BP_SplinePathForSnake.BP_SplinePathForSnake_C" "SnakePath"))
  (if (Utilities|Array|IsNotEmpty _outactors)
    (Variables|Default|SetSnakeSplinePath (Variables|/Game/Blueprints/BP_SplinePathForSnake.BP_SplinePathForSnake_C|GetSpline (Utilities|Array|Get(acopy) _outactors)))
    (Variables|Default|SetPathActorLocation (Transformation|GetActorLocation (Utilities|Array|Get(acopy) _outactors)))
    (Development|PrintString "Found Snake Path....")
    (else
      (Utilities|FlowControl|Delay 0.2)
      (CallFunction|FindSnakePath))))

(event Custom|MoveAlongPath)

(event EventBeginPlay)

(event EventTick
  (params (DeltaSeconds :type Float%20%28single-precision%29)))

(fn ConstructionScript)